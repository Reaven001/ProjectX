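; BP_Asensor is a trigger Blueprint that moves its static mesh along a timeline path, apparently as an elevator.
; EnterEvent enables player 0 input on the actor, then after a short delay plays the timeline that drives the mesh's relative location without sweeping.
; ExitEvent disables that input and, after a longer delay, reverses the timeline to return the mesh.
; The graph itself binds no input actions.
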(event EventExitEvent
  (Input|DisableInput (Game|GetPlayerController 0))
  (Utilities|FlowControl|Delay 1.0)
  (bind _newtrack_1 (Timeline|Timeline_0 Reverse)
    (:Update
      (Transformation|SetRelativeLocation (Variables|Default|GetStaticMesh) _newtrack_1 false false))))

(event EventEnterEvent
  (Input|EnableInput (Game|GetPlayerController 0))
  (Utilities|FlowControl|Delay 0.5)
  (bind _newtrack_1 (Timeline|Timeline_0 Play)
    (:Update
      (Transformation|SetRelativeLocation (Variables|Default|GetStaticMesh) _newtrack_1 false false))))

(fn ConstructionScript
  (|CallParentFunction))